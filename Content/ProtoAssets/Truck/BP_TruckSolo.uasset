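; BP_TruckSolo is a prototype truck actor that drives its static mesh in a continuous circle around a Center component.
; Each Tick places the mesh opposite its right vector from Center's relative location, at a distance of Speed times Radius, used as a world position.
; It then adds Speed to the mesh's relative yaw, so motion is frame-rate dependent and Speed affects both turn rate and orbit size.
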(event `self.ReceiveTick`
  (params (DeltaSeconds :type "Float (single-precision)"))
  (bind _staticmesh (`self.StaticMesh`))
  (bind (_relativerotation_roll _relativerotation_pitch _relativerotation_yaw) (`KismetMathLibrary.BreakRotator` (`SceneComponent.RelativeRotation` _staticmesh)))
  (`SceneComponent.K2_SetWorldLocation` _staticmesh (+ (`SceneComponent.RelativeLocation` (`self.Center`)) (* (* (`SceneComponent.GetRightVector` (`self.StaticMesh`)) -1.0) (`self.Speed`) (`self.Radius`))) false false)
  (`SceneComponent.K2_SetRelativeRotation` _staticmesh (`KismetMathLibrary.MakeRotator` _relativerotation_roll _relativerotation_pitch (+ _relativerotation_yaw (`self.Speed`))) false false))

(fn `UserConstructionScript`)