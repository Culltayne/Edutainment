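; Game instance that holds player stats, background-music state and the GPT conversation transcript.
; Init loads or creates the PlayerStats save and assigns it a fresh UUID, which AppendUUID adds to the username once.
; Coin, XP and music updates write straight to that save slot.
; SaveTranscript flattens user and assistant messages into a string, writes it to Transcript.txt and spawns a GPTSummarizer actor to summarize it.
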(event `UpdateTranscript`
  (params (GPTConversation :type "GPTChatPromptParams Structure"))
  (set `self.GPTConversation` GPTConversation))

(event `SaveTranscript`
  (for _array_element (`.Messages` (break `GPTChatPromptParams` (`self.GPTConversation`)))
    (bind ((`Role` _role) (`UserMessage` _usermessage) (`AssistantMessage` _assistantmessage)) (break `GPTChatMessage` _array_element))
    (switch `EGPTRole` _role
      (:`user`
        (bind (_role_2 _content) (break `UserMessage` _usermessage))
        (set `self.ConvoString` (`KismetStringLibrary.Concat_StrStr` (`self.ConvoString`) (`KismetStringLibrary.Concat_StrStr` _role_2 ": " (`.Content` (break `ContentPart` (`|GetArrayItem` _content))) " \n"))))
      (:`assistant`
        (bind ((`Role` _role_3) (`Content` _content_2)) (break `AssistantMessage` _assistantmessage))
        (set `self.ConvoString` (`KismetStringLibrary.Concat_StrStr` (`self.ConvoString`) (`KismetStringLibrary.Concat_StrStr` _role_3 ": " _content_2 " \n"))))))
  (`FileSDKBPLibrary.WriteStringToFile` (`KismetStringLibrary.Concat_StrStr` (`KismetSystemLibrary.GetProjectSavedDirectory`) "Transcript.txt") (`self.ConvoString`))
  (`self.GenerateSummary`))

(event `GenerateSummary`
  (bind _returnvalue (`|SpawnActorFromClass` "/Game/Blueprints/KalebsFolder/GPTSummarizer.GPTSummarizer_C" (`KismetMathLibrary.MakeTransform` (0.0 0.0 0.0)) "AlwaysSpawn" "MultiplyWithRoot" null null))
  (`/Game/Blueprints/KalebsFolder/GPTSummarizer.GenerateGPTSummary` _returnvalue (`self.ConvoString`)))

(event `AppendUUID`
  ;[0.03466 0.0487 0.15 0.5] Add User name
  (`/Engine/EditorBlueprintResources/StandardMacros.DoOnce` false
    (:`Completed`
      (set `self.Username` (`KismetStringLibrary.Concat_StrStr` (`self.Username`) "_" (`/Game/Blueprints/Core/SaveGames/SG_PlayerStats.UUID` (`self.PlayerStats_Save`)))))))

(event `self.ReceiveInit`
  (`|ExecutionSequence`
    (:`then_0`
      ; Load Player Stats (Coins / XP)
      (bind _returnvalue (`GameplayStatics.DoesSaveGameExist` "PlayerStats"))
      (if _returnvalue
        (bind _returnvalue_2 (`GameplayStatics.LoadGameFromSlot` "PlayerStats"))
        (bind _assg_player_stats (cast `/Game/Blueprints/Core/SaveGames/SG_PlayerStats` _returnvalue_2)
          (:`then`
            (set `self.PlayerStats_Save` _assg_player_stats))
          (:`CastFailed`
            (bind _returnvalue_3 (`GameplayStatics.CreateSaveGameObject` "/Game/Blueprints/Core/SaveGames/SG_PlayerStats.SG_PlayerStats_C" :!label _label))
            (bind _output_get (set `self.PlayerStats_Save` _returnvalue_3))
            (`GameplayStatics.SaveGameToSlot` _output_get "PlayerStats")))
        (else
          (goto _label))))
    (:`then_1`
      ; Set Username
      (set `/Game/Blueprints/Core/SaveGames/SG_PlayerStats.UUID` (`KismetGuidLibrary.Conv_GuidToString` (`KismetGuidLibrary.NewGuid`)) (`self.PlayerStats_Save`)))))

(event `SaveBGMTimestamp`
  (params (Timestamp :type "Float (double-precision)"))
  (bind _playerstats_save (`self.PlayerStats_Save`))
  ; BGM
  (set `/Game/Blueprints/Core/SaveGames/SG_PlayerStats.Timestamp` Timestamp _playerstats_save)
  (`GameplayStatics.SaveGameToSlot` _playerstats_save "PlayerStats"))

(event `SaveBGMState`
  (params (`Playing?` :type Boolean))
  (bind _playerstats_save (`self.PlayerStats_Save`))
  ; BGM
  (set `/Game/Blueprints/Core/SaveGames/SG_PlayerStats.BGMPlaying? ` `Playing?` _playerstats_save)
  (`GameplayStatics.SaveGameToSlot` _playerstats_save "PlayerStats"))

(event `EraseBGMSave`
  (bind _playerstats_save (`self.PlayerStats_Save`))
  ; BGM
  (set `/Game/Blueprints/Core/SaveGames/SG_PlayerStats.Timestamp` 0.0 _playerstats_save)
  (set `/Game/Blueprints/Core/SaveGames/SG_PlayerStats.BGMPlaying? ` true _playerstats_save)
  (`GameplayStatics.SaveGameToSlot` _playerstats_save "PlayerStats"))

(event `UpdatePlayerStats`
  (params (Coins :type Integer) (`XP To Add` :type Integer) (`Removing Coins?` :type Boolean :default true))
  (bind _playerstats_save (`self.PlayerStats_Save`))
  (bind _playerstats_save_2 (`self.PlayerStats_Save`))
  ; Update Player Stats (Coins / XP)
  (if (not `Removing Coins?`)
    (set `/Game/Blueprints/Core/SaveGames/SG_PlayerStats.Coins` (+ Coins (`/Game/Blueprints/Core/SaveGames/SG_PlayerStats.Coins` _playerstats_save)) _playerstats_save)
    (set `/Game/Blueprints/Core/SaveGames/SG_PlayerStats.XP` (+ `XP To Add` (`/Game/Blueprints/Core/SaveGames/SG_PlayerStats.XP` _playerstats_save)) _playerstats_save)
    (else
      (set `/Game/Blueprints/Core/SaveGames/SG_PlayerStats.Coins` (- (`/Game/Blueprints/Core/SaveGames/SG_PlayerStats.Coins` _playerstats_save_2) Coins) _playerstats_save_2)))
  (`GameplayStatics.SaveGameToSlot` _playerstats_save "PlayerStats"))