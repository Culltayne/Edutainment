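; BP_Transition is a level-flow actor that plays the current level's lecture video, then hands off to a GPT assistant or a minigame.
; On BeginPlay it looks up the level name in DT_LevelSetup, with an error-labelled fallback, and opens a video player widget.
; When the video finishes, GPTPrompt selects spawning BP_ResponseGPTAssistant or displaying the MinigameWidgets entry at MinigameCounter, identified by a cast chain, then incrementing the counter.
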(event `self.ReceiveBeginPlay`
  (bind _returnvalue (`GameplayStatics.GetCurrentLevelName` true))
  (bind _returnvalue_2 (`|GetDataTableRow` "/Game/Widgets/VideoPlayer/DT_LevelSetup.DT_LevelSetup" (`KismetStringLibrary.Conv_StringToName` _returnvalue))
    (:`then`
      (set `self.Level Setup` _returnvalue_2)
      (`self.CreateVideoWidget`))
    (:`RowNotFound`
      (set `self.Level Setup` (make `/Game/Widgets/VideoPlayer/S_LevelSetUp` "/Game/Movies/Edutainment_Lecture_1_1_Compositing_Video_White.Edutainment_Lecture_1_1_Compositing_Video_White" "/Game/Movies/Audio/Edutainment_Audio_1_1.Edutainment_Audio_1_1" "Error: Unrecognized level / data table row not found." "Error: Unrecognized level / data table row not found."))
      (`self.CreateVideoWidget`)))
  (set `self.NumberOfMinigames` (`KismetArrayLibrary.Array_Length` (`self.Minigame Widgets`))))

(event `CreateVideoWidget`
  (bind (_video _audio) (break `/Game/Widgets/VideoPlayer/S_LevelSetUp` (`self.Level Setup`)))
  (bind _returnvalue (`|CreateWidget` "/Game/Widgets/VideoPlayer/WBP_UpdatedVideoPlayer.WBP_UpdatedVideoPlayer_C" (`GameplayStatics.GetPlayerController` 0) _video _audio))
  (set `self.Video Player` _returnvalue)
  (`UserWidget.AddToViewport` _returnvalue 0)
  (add `/Game/Widgets/VideoPlayer/WBP_UpdatedVideoPlayer.Video Finished` _returnvalue (delegate `Video Finished`)))

(event `Video Finished`
  (if (`self.GPT Prompt?`)
    (`self.Spawn GPT`)
    (elif (>= (`self.NumberOfMinigames`) (`self.MinigameCounter`))
      (`self.Find Widget` (`self.MinigameCounter`))
      (bind _result (`/Engine/EditorBlueprintResources/StandardMacros.IncrementInt` (`self.MinigameCounter`))
        (:`  `
          (set `self.MinigameCounter` _result))))))

(fn `Find Widget`
  (params (Index :type Integer))
  (bind _output (`|GetArrayItem` (`self.Minigame Widgets`) Index))
  (bind _aswbp_swiping_game (cast `/Game/Widgets/MiniGames/SwipingMini/WBP_SwipingGame` _output)
    (:`then`
      (`UserWidget.AddToViewport` _aswbp_swiping_game 0))
    (:`CastFailed`
      (bind _aswbp_contradiction_game (cast `/Game/Widgets/MiniGames/ContradictionMini/WBP_ContradictionGame` _output)
        (:`then`
          (`UserWidget.AddToViewport` _aswbp_contradiction_game 0))
        (:`CastFailed`
          (bind _aswbp_matching_game (cast `/Game/Widgets/MiniGames/MatchingMini/WBP_MatchingGame` _output)
            (:`then`
              (`UserWidget.AddToViewport` _aswbp_matching_game 0))
            (:`CastFailed`
              (bind _aswbp_categories_game (cast `/Game/Widgets/MiniGames/CategoriesMini/WBP_CategoriesGame` _output)
                (:`then`
                  (`UserWidget.AddToViewport` _aswbp_categories_game 0))
                (:`CastFailed`
                  (bind _aswbp_dialogue_display (cast `/Game/Widgets/MiniGames/Dialogue/WBP_DialogueDisplay` _output)
                    (:`then`
                      (`UserWidget.AddToViewport` _aswbp_dialogue_display 0))
                    (:`CastFailed`
                      (`KismetSystemLibrary.PrintString` "Minigame widget missing or not recognized." true true (struct :`R` 1.0 :`B` 0.021864 :`A` 1.0) 10.0))))))))))))

(fn `Spawn GPT`
  (`|SpawnActorFromClass` "/Game/Blueprints/GPT/BP_ResponseGPTAssistant.BP_ResponseGPTAssistant_C" (`KismetMathLibrary.MakeTransform` (0.0 0.0 0.0)) "Undefined" "MultiplyWithRoot" null null))

(fn `UserConstructionScript`)