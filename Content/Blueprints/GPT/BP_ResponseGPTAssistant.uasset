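; GPT-driven legal coach actor that quizzes a learner on a lecture prompt through a chat widget.
; Typed or Whisper-transcribed messages go to GPT via AIITKComponentBP, streaming replies into the widget and optionally voicing them through ElevenLabs when Talk is on.
; A "Prompt Completed" phrase, requested by the system prompt, reveals the next-level button.
; A GPT_Event completion argument triggers BSOD or fire effects; the color-change handler is empty.
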(event `Activate`
  (bind _returnvalue (`|CreateWidget` "/Game/Widgets/GPT/WBP_ResponseGPTAssistant.WBP_ResponseGPTAssistant_C"))
  (bind _output_get (set `self.ChatInterfaceWidgetRef` _returnvalue))
  (`UserWidget.AddToViewport` _output_get 0)
  (set `/Game/Widgets/GPT/WBP_ResponseGPTAssistant.ShowSystemMessages` (`self.ShowSystemMessages`) _output_get)
  (set `/Game/Widgets/GPT/WBP_ResponseGPTAssistant.ResponseGPTRef` self _output_get))

(event `self.ReceiveBeginPlay`
  ;[0 0 0] Init
  (`KismetSystemLibrary.Delay` 0.2)
  (`|ExecutionSequence`
    (:`then_0`
      (`AIITKDeveloperSettings.SetAPIKey` "OpenAI" (`AIITK_NTK_NetworkingToolkitSettings.GetDecryptedKey` "OpenAI"))
      (`AIITKDeveloperSettings.SetAPIKey` "Labs11" (`AIITK_NTK_NetworkingToolkitSettings.GetDecryptedKey` "11Labs")))
    (:`then_1`
      (`self.AddSystemMessage` (`self.GPTInstructions`) (`self.GPTPrompt`)))
    (:`then_2`
      (set `PlayerController.bShowMouseCursor` true (`GameplayStatics.GetPlayerController` 0))
      (`self.Activate`))))

(event `ToggleRecording`
  ;[0 0 0] Capture voice
  (set `self.Talk? ` (not (`self.Talk? `))))

(event `Send Message`
  ;[0 0 0] Request
  (`self.AddUserMessage`)
  (`/AIIntegrationToolkit/Core/Components/AIITKComponentBP.SendRequestToGPT` (`self.AIITKComponentBP`) (`self.GPTParams`)))

(event `self.AIITKComponentBP.OnAudioCaptureSaved`
  (params (WAVFilePath :type String))
  ;[0 0 0] Whisper request
  (bind _structout (setmembers `WhisperAPIParams` :`StructRef` (`self.WhisperParams`) :`FilePath` WAVFilePath))
  (`/AIIntegrationToolkit/Core/Components/AIITKComponentBP.SendRequestToWhisper` (`self.AIITKComponentBP`) _structout))

(event `Send Message From Voice`
  (params (`User Message` :type String))
  (`self.AddUserMessageFromVoice` `User Message`)
  (`/AIIntegrationToolkit/Core/Components/AIITKComponentBP.SendRequestToGPT` (`self.AIITKComponentBP`) (`self.GPTParams`)))

(event `self.AIITKComponentBP.OnWhisperTranscriptGenerated`
  (params (Transcription :type String))
  ;[0 0 0] Whisper response
  (`self.Send Message From Voice` Transcription))

(event `self.AIITKComponentBP.OnGPTChunkReceived`
  (params (Completion :type "GPTChatCompletion Structure"))
  ;[0 0 0] Responses
  (bind _responsecontent (`self.GetFirstChoiceContent` Completion))
  (`/Game/Widgets/GPT/WBP_ResponseGPTAssistant.UpdateLastMessageOnScreen` (`self.ChatInterfaceWidgetRef`) _responsecontent))

(event `self.AIITKComponentBP.OnGPTFailed`
  (params (ErrorMessage :type "GPTChatCompletion Structure"))
  ;[0 0 0] Responses
  (`self.AddResponseMessage` ErrorMessage))

(event `self.AIITKComponentBP.OnGPTModelsRetrieved`
  (params (ModelIds :type "Array of String (by ref)"))
  ;[0 0 0] Responses
  (`/Game/Widgets/GPT/WBP_ResponseGPTAssistant.UpdateMessagesOnScreen` (`self.ChatInterfaceWidgetRef`) (`self.ModelIdsToMessage` ModelIds)))

(event `self.AIITKComponentBP.OnGPTCompleted`
  (params (Completion :type "GPTChatCompletion Structure"))
  (bind _currentchatcompletion (`self.CurrentChatCompletion`))
  (bind _returnvalue (`OpenAIFunctionLibrary.GetMessageContent` (`OpenAIFunctionLibrary.GetResponseMessage` Completion)))
  (`|ExecutionSequence`
    (:`then_0`
      (bind _output_get (set `self.CurrentChatCompletion` Completion))
      (if (`self.Talk? `)
        (bind _structout (setmembers `11LabsRequestParams` :`StructRef` (`self.11LabsRequest`) :`TextPrompt` (`OpenAIFunctionLibrary.GetMessageContent` (`OpenAIFunctionLibrary.GetResponseMessage` _output_get))))
        (bind _11labsinstance (`/AIIntegrationToolkit/Core/Components/AIITKComponentBP.SendRequestTo11Labs` (`self.AIITKComponentBP`) _structout))
        (add `TextToSpeechAPI.OnAudioWithAlignmentGenerated` _11labsinstance (`|CreateDelegate` :!event `AudioRecieved`))
        (else
          (`self.AddResponseMessage` (`self.CurrentChatCompletion`))))
      (`self.RunFunctionLogic` _currentchatcompletion)
      (`self.LogCompletion` _currentchatcompletion))
    (:`then_1`
      (bind _output_get_2 (set `self.IsCompleted` (== (`KismetStringLibrary.GetSubstring` _returnvalue (`KismetStringLibrary.FindSubstring` _returnvalue "Prompt Completed" false true) 16) "Prompt Completed")))
      (if _output_get_2
        (`self.PromptCompleted`)))))

(event `PromptCompleted`
  (bind _chatinterfacewidgetref (`self.ChatInterfaceWidgetRef`))
  ;[1 0.5389 0.06424] When GPT says you've learned enough, let's show the close button and the next level button
  ; (also do this when there IS no prompt)
  ; These are set to invisible on begin play
  (`Widget.SetVisibility` (`/Game/Widgets/GPT/WBP_ResponseGPTAssistant.Btn_NextLevel` _chatinterfacewidgetref) "Visible")
  (`Widget.SetVisibility` (`/Game/Widgets/GPT/WBP_ResponseGPTAssistant.Btn_NextLevel` _chatinterfacewidgetref) "Visible"))

(fn `AddResponseMessage`
  (params (ChatCompletion :type "GPTChatCompletion Structure (by ref)"))
  (bind _gptparams (`self.GPTParams`))
  (`KismetArrayLibrary.Array_Add` (`.Messages` (break `GPTChatPromptParams` (`self.GPTParams`))) (`OpenAIFunctionLibrary.GetResponseMessage` ChatCompletion))
  (`/Game/Widgets/GPT/WBP_ResponseGPTAssistant.UpdateMessagesOnScreen` (`self.ChatInterfaceWidgetRef`) _gptparams)
  (`/AIIntegrationToolkit/Core/Components/AIITKComponentBP.TruncateMessages` (`self.AIITKComponentBP`) _gptparams))

(fn `AddSystemMessage`
  (params (Content :type String) (Prompt :type String))
  (`KismetArrayLibrary.Array_Add` (`.Messages` (break `GPTChatPromptParams` (`self.GPTParams`))) (make `GPTChatMessage` "system" "" (make `SystemMessage` "system" (`KismetTextLibrary.Conv_TextToString` (`|FormatText` "You are a legal coach. \nThe learner was given this prompt: {Prompt} \nThe learner was given these instructions: {Instructions} \nYour task is provided in the instructions. \n \nIf you believe that they correctly answered the prompt and all follow up questions, end your response with \"Prompt Completed\".  Only do this when you are done asking them questions and you believe they understand the subject, because saying \"Prompt Completed\" will allow the user to end your conversation with them. DO NOT answer the question for them.  *ONLY* say \"Prompt Completed\" when *THEY* answer all the questions correctly.  It is important that you let them come to conclusions.  After saying \"Prompt Completed,\" tell the user they may continue to the next section of the lecture." Prompt Content))) (struct :`Role` "user") (make `AssistantMessage` ""))))

(fn `AddUserMessage`
  (bind _chatinterfacewidgetref (`self.ChatInterfaceWidgetRef`))
  (`KismetArrayLibrary.Array_Add` (`.Messages` (break `GPTChatPromptParams` (`self.GPTParams`))) (make `GPTChatMessage` :`Role` "user" :`UserMessage` (make `UserMessage` (`|MakeArray` (make `ContentPart` "Text" (`KismetTextLibrary.Conv_TextToString` (`MultiLineEditableText.GetText` (`/Game/Widgets/GPT/WBP_ResponseGPTAssistant.UserPrompt` (`self.ChatInterfaceWidgetRef`))))) :!type "ContentPart Structure"))))
  (`/Game/Widgets/GPT/WBP_ResponseGPTAssistant.UpdateMessagesOnScreen` _chatinterfacewidgetref (`self.GPTParams`))
  (`/Game/Widgets/GPT/WBP_ResponseGPTAssistant.ClearUserPrompt` _chatinterfacewidgetref)
  (`/Game/Widgets/GPT/WBP_ResponseGPTAssistant.AddNewChatObject` (`self.ChatInterfaceWidgetRef`) (make `GPTChatMessage` "assistant")))

(fn `AddUserMessageFromVoice`
  (params (`User Message` :type String))
  (`KismetArrayLibrary.Array_Add` (`.Messages` (break `GPTChatPromptParams` (`self.GPTParams`))) (make `GPTChatMessage` :`Role` "user" :`UserMessage` (make `UserMessage` (`|MakeArray` (make `ContentPart` "Text" `User Message`) :!type "ContentPart Structure"))))
  (`/Game/Widgets/GPT/WBP_ResponseGPTAssistant.UpdateMessagesOnScreen` (`self.ChatInterfaceWidgetRef`) (`self.GPTParams`))
  (`/Game/Widgets/GPT/WBP_ResponseGPTAssistant.AddNewChatObject` (`self.ChatInterfaceWidgetRef`) (make `GPTChatMessage` "system")))

(fn `AudioRecieved`
  (params (GeneratedAudio :type "SoundWave Object Reference") (AlignmentData :type "CharacterAlignment Structure (by ref)"))
  (bind _speaker (`self.Speaker`))
  (if (`AudioComponent.IsPlaying` (`self.Speaker`))
    (`self.StopCurrentSound`)
    (else
      (`self.AddResponseMessage` (`self.CurrentChatCompletion`))))
  (`/Game/Widgets/GPT/WBP_ResponseGPTAssistant.AudioStarted` (`self.ChatInterfaceWidgetRef`))
  (`AudioComponent.SetSound` _speaker GeneratedAudio)
  (`AudioComponent.Play` _speaker 0.0)
  (return))

(fn `StopCurrentSound`
  (`AudioComponent.Stop` (`self.Speaker`))
  (`/Game/Widgets/GPT/WBP_ResponseGPTAssistant.AudioEnded` (`self.ChatInterfaceWidgetRef`))
  (return))

(fn `UserConstructionScript`)