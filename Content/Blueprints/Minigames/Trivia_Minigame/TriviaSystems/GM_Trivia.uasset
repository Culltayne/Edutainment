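; GM_Trivia is the trivia minigame's game mode, which picks questions from a category and sends them to players.
; A temporary test hook in PostLogin starts the LAW1 category once after a short delay, shuffling its question pool.
; AskQuestion saves the correct answer before shuffling the choices, then passes the question and shuffled choices to each player's PC_Trivia controller.
; The file neither advances the question index nor checks answers.
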(event `self.K2_PostLogin`
  (params (NewPlayer :type "PlayerController Object Reference"))
  (`KismetSystemLibrary.Delay` 3.0)
  ; Temporary for testing
  (`/Engine/EditorBlueprintResources/StandardMacros.DoOnce` false
    (:`Completed`
      (`self.BeginCategory` "/Game/Blueprints/Minigames/Trivia_Minigame/LawQuestions/Category_LAW1.Category_LAW1"))))

(event `BeginCategory`
  (params (Category :type "/Game/Blueprints/Minigames/Trivia_Minigame/DA_Category Object Reference"))
  (bind _output_get (set `self.CurrentCategory` Category))
  (bind _output_get_2 (set `self.CurrentQuestionPool` (`/Game/Blueprints/Minigames/Trivia_Minigame/DA_Category.QuestionPool` _output_get)))
  (`KismetArrayLibrary.Array_Shuffle` _output_get_2)
  (`self.AskQuestion`))

(event `AskQuestion`
  (bind _output (`|GetArrayItem` (`self.CurrentQuestionPool`) (`self.CurrentQuestionIndex`)))
  (bind _multiplechoice (`/Game/Blueprints/Minigames/Trivia_Minigame/DA_Question.MultipleChoice` _output))
  (set `self.CorrectAnswer` (`|GetArrayItem` _multiplechoice (`/Game/Blueprints/Minigames/Trivia_Minigame/DA_Question.CorrectAnswer` _output)))
  (bind _output_get (set `self.CurrentMultipleChoice` _multiplechoice))
  (`KismetArrayLibrary.Array_Shuffle` _output_get)
  (for _array_element (`GameStateBase.PlayerArray` (`GameplayStatics.GetGameState`))
    (bind _aspc_trivia (cast `/Game/Blueprints/Minigames/Trivia_Minigame/TriviaSystems/PC_Trivia` (`PlayerState.GetPlayerController` _array_element)))
    (`/Game/Blueprints/Minigames/Trivia_Minigame/TriviaSystems/PC_Trivia.AskQuestion` _aspc_trivia (`|GetArrayItem` (`self.CurrentQuestionPool`) (`self.CurrentQuestionIndex`)) (`self.CurrentMultipleChoice`))))

(fn `UserConstructionScript`)