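; Player controller for the trivia minigame that relays questions, answers and reveals between the player's HUD and the game state.
; Asking a question starts a fixed question timer and shows it on HUD_Trivia, while submitted answers go to GS_Trivia with the time remaining.
; On timer expiry it checks every player's controller timer and triggers the client answer reveal only when none remain active.
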(event `self.ReceiveBeginPlay`
  (`WidgetBlueprintLibrary.SetInputMode_UIOnlyEx` self null))

(event `AskQuestion`
  (params (Question :type "/Game/Blueprints/Minigames/Trivia_Minigame/DA_Question Object Reference") (MultipleChoice :type "Array of Text"))
  (`self.StartTimer`)
  (bind _ashud_trivia (cast `/Game/Blueprints/Minigames/Trivia_Minigame/TriviaSystems/HUD_Trivia` (`self.GetHUD`)))
  (`/Game/Blueprints/Minigames/Trivia_Minigame/TriviaSystems/HUD_Trivia.AskQuestion` _ashud_trivia Question MultipleChoice))

(event `CLIENT_RevealAnswers`
  (bind _ashud_trivia (cast `/Game/Blueprints/Minigames/Trivia_Minigame/TriviaSystems/HUD_Trivia` (`self.GetHUD` (`GameplayStatics.GetPlayerController` 0))))
  (`/Game/Blueprints/Minigames/Trivia_Minigame/TriviaSystems/HUD_Trivia.RevealAnswers` _ashud_trivia))

(event `SetAnswer`
  (params (Answer :type Text) (TimeRemaining :type "Float (double-precision)"))
  (bind _asgs_trivia (cast `/Game/Blueprints/Minigames/Trivia_Minigame/TriviaSystems/GS_Trivia` (`GameplayStatics.GetGameState`)))
  (`/Game/Blueprints/Minigames/Trivia_Minigame/TriviaSystems/GS_Trivia.MC_UpdateLockedInAnswers` _asgs_trivia (`self.PlayerState`) Answer TimeRemaining))

(event `TimerExpired`
  (bind _return (`self.CheckTimerStatus`))
  (if _return
    (`self.CLIENT_RevealAnswers`)))

(fn `CheckTimerStatus`
  (returns (Return :type Boolean))
  (for _array_element (`GameStateBase.PlayerArray` (`GameplayStatics.GetGameState`))
    (bind _aspc_trivia (cast `/Game/Blueprints/Minigames/Trivia_Minigame/TriviaSystems/PC_Trivia` (`PlayerState.GetPlayerController` _array_element)))
    (if (`KismetSystemLibrary.K2_IsTimerActiveHandle` (`/Game/Blueprints/Minigames/Trivia_Minigame/TriviaSystems/PC_Trivia.QuestionTimer` _aspc_trivia))
      (return false)))
  (return true))

(fn `StartTimer`
  (bind _returnvalue (`KismetSystemLibrary.K2_SetTimerDelegate` (`|CreateDelegate` :!event `TimerExpired`) 10.0))
  (set `self.QuestionTimer` _returnvalue))

(fn `UserConstructionScript`)